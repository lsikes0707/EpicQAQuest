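; BP_Elevator is an elevator whose platform starts moving when a BP_ThirdPersonCharacter overlaps its CheckForPlayerTrigger component.
; Two timelines, one played from start and one reversed from end, drive the platform's relative Z across a fixed travel height.
; Each timeline's finish starts the other, so the platform cycles up and down endlessly with no stop logic.
; Every new overlap calls the raise again from its start, with no guard.
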(event `self.ReceiveBeginPlay`)

(event `ElevatorRaiseCustomEvent`
  (bind (_direction _raise_elevator_value) (`Timeline|ElevatorUp` :!via `PlayFromStart`)
    (:`Update`
      (`SceneComponent.K2_SetRelativeLocation` (`self.ElevatorPlatform`) (`KismetMathLibrary.MakeVector` 0.0 0.0 (* _raise_elevator_value 2030.0)) false false))
    (:`Finished`
      (`self.ElevatorLowerCustomEvent`))))

(event `ElevatorLowerCustomEvent`
  (bind (_direction _lower_elevator_value) (`Timeline|ElevatorLower` :!via `ReverseFromEnd`)
    (:`Update`
      (`SceneComponent.K2_SetRelativeLocation` (`self.ElevatorPlatform`) (`KismetMathLibrary.MakeVector` 0.0 0.0 (* _lower_elevator_value 2030.0)) false false))
    (:`Finished`
      (`self.ElevatorRaiseCustomEvent`))))

(event `TurnElevatorOnCustomEvent`
  (`self.ElevatorRaiseCustomEvent`))

(event `self.CheckForPlayerTrigger.OnComponentBeginOverlap`
  (params (OverlappedComponent :type "PrimitiveComponent Object Reference") (OtherActor :type "Actor Object Reference") (OtherComp :type "PrimitiveComponent Object Reference") (OtherBodyIndex :type Integer) (bFromSweep :type Boolean) (SweepResult :type "HitResult Structure (by ref)"))
  (cast `/Game/ThirdPerson/Blueprints/BP_ThirdPersonCharacter` OtherActor)
  (`self.TurnElevatorOnCustomEvent`))

(fn `UserConstructionScript`)