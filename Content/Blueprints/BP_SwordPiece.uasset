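; BP_SwordPiece is a collectible code piece that shows two text snippets and turns green when the player character enters its trigger box.
; On overlap it sets IsGreen, swaps the backdrop to an emissive material, and has BP_Sword check whether all code pieces are green.
; It then unhides the return portal and the BP_Sword medal directly, without waiting on that check's result.
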(event `self.ReceiveBeginPlay`
  (`TextRenderComponent.K2_SetText` (`self.CodeSnip`) (`KismetTextLibrary.Conv_StringToText` (`self.Code`)))
  (`TextRenderComponent.K2_SetText` (`self.CodeSnip2`) (`KismetTextLibrary.Conv_StringToText` (`self.Code2`))))

(event `self.TriggerBox.OnComponentBeginOverlap`
  (params (OverlappedComponent :type "PrimitiveComponent Object Reference") (OtherActor :type "Actor Object Reference") (OtherComp :type "PrimitiveComponent Object Reference") (OtherBodyIndex :type Integer) (bFromSweep :type Boolean) (SweepResult :type "HitResult Structure (by ref)"))
  (cast `/Game/ThirdPerson/Blueprints/BP_ThirdPersonCharacter` OtherActor)
  (set `self.IsGreen?` true)
  (`PrimitiveComponent.SetMaterial` (`self.CodeBackdrop`) 0 "/Game/Materials/EmmissiveShapeMaterial.EmmissiveShapeMaterial")
  (`self.NotifySword` self)
  ;[1 1 1] Unhide the portal for return to main
  (bind _returnvalue (`GameplayStatics.GetActorOfClass` "/Game/Blueprints/BP_Portal.BP_Portal_C"))
  (`self.SetActorHiddenInGame` _returnvalue false)
  ;[1 1 1] Unhide the medal for the player to collect
  (bind _returnvalue_2 (`GameplayStatics.GetActorOfClass` "/Game/Blueprints/BP_Sword.BP_Sword_C"))
  (`self.SetActorHiddenInGame` _returnvalue_2 false))

(event `NotifySword`
  (bind _outactors (`GameplayStatics.GetAllActorsOfClass` "/Game/Blueprints/BP_Sword.BP_Sword_C"))
  (`/Game/Blueprints/BP_Sword.CheckForAllGreenCodePieces` (`|GetArrayItem` _outactors)))

(fn `UserConstructionScript`)