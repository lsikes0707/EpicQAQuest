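; BP_Sword is a pickup that tells the player they have won a medal and can return through the portal.
; On BeginPlay it sets its visibility from IsHidden.
; When BP_ThirdPersonCharacter overlaps TriggerBox, it prints both messages and destroys itself.
; The check that all BP_SwordPiece code pieces are green is unfinished: its event only fetches one piece, and the loop and spawn nodes are disconnected.
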(event `self.ReceiveBeginPlay`
  (`self.SetActorHiddenInGame` self (`self.IsHidden?`)))

(event `CheckForAllGreenCodePieces`
  ;[1 1 1] Code to revisit when ready to enable all 4 code pieces are triggered before presenting medal and exit.
  (`GameplayStatics.GetActorOfClass` "/Game/Blueprints/BP_SwordPiece.BP_SwordPiece_C"))

(event `self.TriggerBox.OnComponentBeginOverlap`
  (params (OverlappedComponent :type "PrimitiveComponent Object Reference") (OtherActor :type "Actor Object Reference") (OtherComp :type "PrimitiveComponent Object Reference") (OtherBodyIndex :type Integer) (bFromSweep :type Boolean) (SweepResult :type "HitResult Structure (by ref)"))
  (cast `/Game/ThirdPerson/Blueprints/BP_ThirdPersonCharacter` OtherActor)
  (`KismetSystemLibrary.PrintString` "Return through the portal to take on your next challenge." true true (struct :`A` 1.0) 5.0)
  (`KismetSystemLibrary.PrintString` "You've won a medal!" true true (struct :`A` 1.0) 5.0)
  (`self.K2_DestroyActor` (`ActorComponent.GetOwner` (`self.SM_Sword`))))

(fn `UserConstructionScript`)